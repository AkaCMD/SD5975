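; BP_DamageBox is a hazard volume that damages a VRPawn that stays inside its DamageBox component.
; Begin overlap stores the pawn and starts a non-looping one-second timer, whose event applies a fixed amount of damage once.
; End overlap by a VRPawn clears the timer through its stored handle, so leaving early cancels the pending damage.
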(event `self.DamageBox.OnComponentBeginOverlap`
  (params (OverlappedComponent :type "PrimitiveComponent Object Reference") (OtherActor :type "Actor Object Reference") (OtherComp :type "PrimitiveComponent Object Reference") (OtherBodyIndex :type Integer) (bFromSweep :type Boolean) (SweepResult :type "HitResult Structure (by ref)"))
  ; Apply damage
  (bind _asvrpawn (cast `/Game/VRTemplate/Blueprints/VRPawn` OtherActor))
  (set `self.As VRPawn` _asvrpawn)
  (bind _returnvalue (`KismetSystemLibrary.K2_SetTimerDelegate` (delegate `DamagePlayer`) 1.0))
  (set `self.TimerRef` _returnvalue))

(event `DamagePlayer`
  ; Apply damage
  (`GameplayStatics.ApplyDamage` (`self.As VRPawn`) 10.0))

(event `self.DamageBox.OnComponentEndOverlap`
  (params (OverlappedComponent :type "PrimitiveComponent Object Reference") (OtherActor :type "Actor Object Reference") (OtherComp :type "PrimitiveComponent Object Reference") (OtherBodyIndex :type Integer))
  ; Stop applying damage
  (cast `/Game/VRTemplate/Blueprints/VRPawn` OtherActor)
  (`KismetSystemLibrary.K2_ClearAndInvalidateTimerHandle` (`self.TimerRef`)))

(fn `UserConstructionScript`)