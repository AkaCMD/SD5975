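; BP_Fireball is a fireball actor that destroys any actor tagged Enemy that it hits.
; On any hit it spawns an explosion particle at its own location and destroys itself.
; On BeginPlay its Sphere component is set to ignore the first player's character while moving, and a delay destroys the fireball after ten seconds if it still exists.
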(event `self.ReceiveHit`
  (params (MyComp :type "PrimitiveComponent Object Reference") (Other :type "Actor Object Reference") (OtherComp :type "PrimitiveComponent Object Reference") (bSelfMoved :type Boolean) (HitLocation :type "Vector Structure") (HitNormal :type "Vector Structure") (NormalImpulse :type "Vector Structure") (Hit :type "HitResult Structure (by ref)"))
  (if (`self.ActorHasTag` Other "Enemy")
    (`self.K2_DestroyActor` Other))
  (`GameplayStatics.SpawnEmitterAtLocation` "/Game/StarterContent/Particles/P_Explosion.P_Explosion" (`self.K2_GetActorLocation`))
  (`/Engine/EditorBlueprintResources/StandardMacros.IsValid` self
    (:`Is Valid`
      (`self.K2_DestroyActor`))))

(event `self.ReceiveBeginPlay`
  (`PrimitiveComponent.IgnoreActorWhenMoving` (`self.Sphere`) (`GameplayStatics.GetPlayerCharacter` 0) true)
  (`KismetSystemLibrary.Delay` 10.0)
  (`/Engine/EditorBlueprintResources/StandardMacros.IsValid` self
    (:`Is Valid`
      (`self.K2_DestroyActor`))))

(fn `UserConstructionScript`)